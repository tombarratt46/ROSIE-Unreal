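; FlagBP is a placeable flag marker actor that displays its world coordinates on two FlagWidget widget components.
; Each Tick, it passes the Sphere's location to both widgets, scaled to hundredths with Y negated, and destroys itself if either requests deletion.
; IsPlaced controls widget visibility; once placed, both labels show the unscaled X and Y, rounded to two decimals.
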(event `self.ReceiveTick`
  (params (DeltaSeconds :type "Float (single-precision)"))
  (bind _isplaced (`self.isPlaced`))
  (bind (_returnvalue_x _returnvalue_y) (`KismetMathLibrary.BreakVector` (`SceneComponent.K2_GetComponentLocation` (`self.Sphere`))))
  (bind _returnvalue (* (`SceneComponent.K2_GetComponentLocation` (`self.Sphere`)) (0.01 -0.01 0.01)))
  (bind _returnvalue_2 (`KismetTextLibrary.Conv_StringToText` (`KismetStringLibrary.Concat_StrStr` "Coordinates: X = " (`KismetStringLibrary.Conv_DoubleToString` (/ (`KismetMathLibrary.Conv_IntToDouble` (`KismetMathLibrary.Round` (* _returnvalue_x 100.0))) 100.0)) ", Y = " (`KismetStringLibrary.Conv_DoubleToString` (/ (`KismetMathLibrary.Conv_IntToDouble` (`KismetMathLibrary.Round` (* _returnvalue_y 100.0))) 100.0)))))
  (bind _asflag_widget (cast `/Game/FlagWidget` (`WidgetComponent.GetWidget` (`self.Widget1`))))
  (set `/Game/FlagWidget.position` _returnvalue _asflag_widget)
  (bind _asflag_widget_2 (cast `/Game/FlagWidget` (`WidgetComponent.GetWidget` (`self.Widget`))))
  (set `/Game/FlagWidget.position` _returnvalue _asflag_widget_2)
  (bind _asflag_widget_3 (cast `/Game/FlagWidget` (`WidgetComponent.GetWidget` (`self.Widget1`))))
  (bind _asflag_widget_4 (cast `/Game/FlagWidget` (`WidgetComponent.GetWidget` (`self.Widget`))))
  (if (or (`/Game/FlagWidget.toDelete` _asflag_widget_3) (`/Game/FlagWidget.toDelete` _asflag_widget_4))
    (`self.K2_DestroyActor`)
    (else
      (`SceneComponent.SetVisibility` (`self.Widget1`) _isplaced false)
      (`SceneComponent.SetVisibility` (`self.Widget`) _isplaced true)
      (if _isplaced
        (bind _asflag_widget_5 (cast `/Game/FlagWidget` (`WidgetComponent.GetWidget` (`self.Widget`)))
          (:`then`
            (set `TextBlock.Text` _returnvalue_2 (`/Game/FlagWidget.TextBlock_Coordinates` _asflag_widget_5))
            (bind _asflag_widget_6 (cast `/Game/FlagWidget` (`WidgetComponent.GetWidget` (`self.Widget1`))))
            (set `TextBlock.Text` _returnvalue_2 (`/Game/FlagWidget.TextBlock_Coordinates` _asflag_widget_6)))
          (:`CastFailed`
            (`KismetSystemLibrary.PrintString` "Ayo")))))))

(fn `UserConstructionScript`)